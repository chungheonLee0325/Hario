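; Field system actor that spawns and triggers a Chaos master field at its own location as soon as play begins.
; BeginPlay spawns FS_MasterField at the actor's transform, sets its activation type and calls CETrigger.
; An unconnected older setup that applies radial cluster strain and linear force through its own FieldSystemComponent remains in the graph but never runs.
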(event EventBeginPlay
  (bind _returnvalue (Game|SpawnActorfromClass "/Engine/EditorResources/FieldNodes/FS_MasterField.FS_MasterField_C" (Transformation|GetActorTransform) "AlwaysSpawn" "MultiplyWithRoot" 0 0))
  (Variables|/Engine/EditorResources/FieldNodes/FS_MasterField.FS_MasterField_C|SetActivationType _returnvalue "NewEnumerator2")
  (Default|CETrigger _returnvalue))

(event Collision|EventActorBeginOverlap
  (params (OtherActor :type Actor%20Object%20Reference)))

(event EventTick
  (params (DeltaSeconds :type Float%20%28single-precision%29)))

(fn ConstructionScript)