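; BP_Player_Mario is the Mario player Blueprint, handling input mode setup and the lose screen on death.
; On BeginPlay it switches the first player controller to Game and UI input and shows the mouse cursor.
; Its Die event creates the HUD_GameOver widget, adds it to the viewport and sets its state text to show that the player lost.
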(event EventBeginPlay
  (bind _returnvalue (Game|GetPlayerController 0))
  (Input|SetInputModeGameandUI _returnvalue 0 "DoNotLock" true false)
  (Variables|/Script/Engine.PlayerController|SetbShowMouseCursor _returnvalue true))

(event Collision|EventActorBeginOverlap
  (params (OtherActor :type Actor%20Object%20Reference)))

(event EventTick
  (params (DeltaSeconds :type Float%20%28single-precision%29)))

(event EventDie
  (bind _returnvalue (UserInterface|CreateWidget "/Game/_BluePrints/Common/UI/Widget/HUD_GameOver.HUD_GameOver_C" (Game|GetPlayerController 0)))
  (UserInterface|Viewport|AddtoViewport _returnvalue 0)
  (Variables|/Script/UMG.TextBlock|SetText (Variables|/Game/_BluePrints/Common/UI/Widget/HUD_GameOver.HUD_GameOver_C|GetGameStateText _returnvalue) "Player Lose"))

(fn ConstructionScript)