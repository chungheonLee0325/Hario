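; BP_AreaObject is a damageable area object actor whose stats come from data keyed by its AreaObjectID.
; On BeginPlay it fetches that data from BP_Hario_GameInstance and initializes its Health component with the data's HP.
; AnyDamage truncates damage and passes it through OnDamaged to Health until OnDie sets the IsDie flag.
; OnSkill is an empty event in this graph.
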(event Custom|OnSkill)

(event Custom|OnDamaged
  (params (Damage :type Integer))
  (if (not (Variables|Status|GetIsDie))
    (Default|TakeDamageHP (Variables|Default|GetHealth) Damage)))

(event Custom|OnDie
  (Variables|Status|SetIsDie true))

(event EventBeginPlay
  (bind _ashario_game_instance (Utilities|Casting|CastToBP_Hario_GameInstance (Game|GetGameInstance)))
  (bind _data (Default|GetAreaObjectData _ashario_game_instance (Variables|Data|GetAreaObjectID)))
  (bind _output_get (Variables|Data|SetData_AreaObject _data))
  (Default|InitHealth (Variables|Default|GetHealth) (.hp _output_get)))

(event Collision|EventActorBeginOverlap
  (params (OtherActor :type Actor%20Object%20Reference)))

(event EventTick
  (params (DeltaSeconds :type Float%20%28single-precision%29)))

(event Game|Damage|EventAnyDamage
  (params (Damage :type Float%20%28single-precision%29) (DamageType :type Damage%20Type%20Object%20Reference) (InstigatedBy :type Controller%20Object%20Reference) (DamageCauser :type Actor%20Object%20Reference))
  (CallFunction|OnDamaged (Math|Float|Truncate Damage)))

(fn ConstructionScript)