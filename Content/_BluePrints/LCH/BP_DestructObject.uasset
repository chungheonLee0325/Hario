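; Breakable object actor that shatters and drops a random pickup when destroyed.
; On the Destruct component's OnDestruction event, it spawns BP_GC_Cube at its own transform and passes the received location to ApplyDestruct.
; It then randomly spawns either a Heart or a BP_CoinStack at ItemDropPosition and destroys itself.
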(event OnDestruction(Destruct)
  (params (ActorLocation :type Vector :default "0, 0, 0"))
  (bind _itemdropposition (Variables|Default|GetItemDropPosition))
  (bind _returnvalue (Transformation|GetWorldLocation _itemdropposition))
  (bind _returnvalue_2 (Game|SpawnActorfromClass "/Game/_BluePrints/LCH/BP_GC_Cube.BP_GC_Cube_C" (Transformation|GetActorTransform) "AlwaysSpawn" "MultiplyWithRoot" 0 0))
  (Default|ApplyDestruct _returnvalue_2 ActorLocation)
  (if (Math|Random|RandomBool)
    (Game|SpawnActorfromClass "/Script/HarioOdyssey.Heart" (Math|Transform|MakeTransform _returnvalue "0, 0, 0" "1.000000,1.000000,1.000000") "Undefined" "MultiplyWithRoot" 0 0)
    (else
      (Game|SpawnActorfromClass "/Game/_BluePrints/Common/BP_CoinStack.BP_CoinStack_C" (Math|Transform|MakeTransform _returnvalue "0, 0, 0" "1.000000,1.000000,1.000000") "Undefined" "MultiplyWithRoot" 0 0)
      (Actor|DestroyActor)))
  (Actor|DestroyActor))

(event EventBeginPlay)

(event Collision|EventActorBeginOverlap
  (params (OtherActor :type Actor%20Object%20Reference)))

(event EventTick
  (params (DeltaSeconds :type Float%20%28single-precision%29)))

(fn ConstructionScript)