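; Boss encounter trigger that spawns an arena and a horde of Burrbo enemies when Player_Mario overlaps it.
; Overlap spawns BP_BossZone and scatters walking Burrbos at random around it, tracking them in Monsters.
; IsStart does not block repeat spawns; boss music plays only on overlaps after it is set.
; Tick prunes invalid monsters, then destroys the zone and shows HUD_GameOver once none remain.
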(event EventBeginPlay)

(event Collision|EventActorBeginOverlap
  (params (OtherActor :type Actor%20Object%20Reference))
  (if (Variables|Default|GetIsStart)
    (bind _ashario_game_mode (Utilities|Casting|CastToHarioGameMode (Game|GetGameMode)))
    (Class|HarioGameMode|PlayBGM _ashario_game_mode 1003 true))
  (Utilities|Casting|CastToPlayer_Mario OtherActor)
  (bind _returnvalue (Game|SpawnActorfromClass "/Game/_BluePrints/LCH/BP_BossZone.BP_BossZone_C" (Variables|Default|GetBossZoneTransform) "AlwaysSpawn" "MultiplyWithRoot" 0 0))
  (for _index (range 0 20)
    (bind _returnvalue_2 (Game|SpawnActorfromClass "/Script/HarioOdyssey.Burrbo" (Math|Transform|MakeTransform (+ (.location (Variables|Default|GetBossZoneTransform)) (* (Class|KismetMathLibrary|VectorNormal2D (Math|Random|RandomUnitVector) 0.0001) (Math|Random|RandomFloatinRange 1e+02 1.7e+03)) "0.000000,0.000000,70.000000") "0, 0, 0" "1.000000,1.000000,1.000000") "Undefined" "MultiplyWithRoot" 0 0))
    (Utilities|Array|Add (Variables|Default|GetMonsters) _returnvalue_2)
    (Pawn|Components|CharacterMovement|SetMovementMode (Variables|/Script/Engine.Character|GetCharacterMovement _returnvalue_2) "MOVE_Walking" 0))
  (Variables|Default|SetIsStart true))

(event EventTick
  (params (DeltaSeconds :type Float%20%28single-precision%29))
  (bind _monsters (Variables|Default|GetMonsters))
  (if (not (or (Variables|Default|GetIsClear) (not (Variables|Default|GetIsStart))))
    (for (_array_element _array_index) _monsters
      (if (not (Utilities|IsValid _array_element))
        (Utilities|Array|RemoveIndex _monsters _array_index)))
    (if (Utilities|Array|IsEmpty _monsters)
      (Actor|DestroyActor (stale Collision|EventActorBeginOverlap _returnvalue))
      (Variables|Default|SetIsClear true)
      (bind _returnvalue (UserInterface|CreateWidget "/Game/_BluePrints/Common/UI/Widget/HUD_GameOver.HUD_GameOver_C" (Game|GetPlayerController 0)))
      (UserInterface|Viewport|AddtoViewport _returnvalue 0))))

(fn ConstructionScript)