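; Health component that tracks maximum and current HP for its owning actor and triggers death.
; InitHealth sets the maximum HP and fills current HP to it.
; TakeDamageHP subtracts damage and, at zero or below, clamps HP to zero and calls OnDie on the owner cast to BP_AreaObject.
; No guard stops OnDie from firing again on later hits.
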(event Custom|TakeDamageHP
  (params (Damage :type Integer))
  ;[0.15 0.15 0.15 0.5] HP 처리
  (bind _output_get (Variables|Default|SetCurrentHP (- (Variables|Default|GetCurrentHP) Damage)))
  ;[0.15 0.15 0.15 0.5] 죽음 처리
  (if (<= _output_get 0)
    (Variables|Default|SetCurrentHP 0)
    (bind _asarea_object (Utilities|Casting|CastToBP_AreaObject (Components|GetOwner)))
    (Default|OnDie _asarea_object)))

(event EventBeginPlay)

(event EventTick
  (params (DeltaSeconds :type Float%20%28single-precision%29)))

(fn InitHealth
  (params (MaxHP :type Integer))
  (bind _output_get (Variables|Data|SetMaxHP MaxHP))
  (Variables|Default|SetCurrentHP _output_get))