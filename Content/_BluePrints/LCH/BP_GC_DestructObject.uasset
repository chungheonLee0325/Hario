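; Destructible Geometry Collection actor that breaks on demand and cleans itself up, destroying itself 4 seconds after BeginPlay regardless of hits.
; ApplyDestruct spawns a BP_FieldSystem 100 units from the actor toward the supplied location, draws debug spheres, then destroys the actor after 2 seconds.
; The wire after DestroyActor loops back to the debug drawing, and several disconnected test chains remain unused.
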(event Custom|ApplyDestruct
  (params (ActorLocation :type Vector))
  (bind _returnvalue (Transformation|GetActorLocation))
  (bind _returnvalue_2 (- ActorLocation _returnvalue))
  (bind _returnvalue_3 (Math|Vector|Normalize _returnvalue_2))
  (bind _returnvalue_4 (* _returnvalue_3 1e+02))
  (bind _returnvalue_5 (+ _returnvalue _returnvalue_4))
  (Game|SpawnActorfromClass "/Game/_BluePrints/LCH/BP_FieldSystem.BP_FieldSystem_C" (Math|Transform|MakeTransform _returnvalue_5 "0, 0, 0" "1.000000,1.000000,1.000000") "AlwaysSpawn" "MultiplyWithRoot" 0 0)
  (Rendering|Debug|DrawDebugSphere _returnvalue_2 2e+02 50 "(R=1.000000,G=0.000000,B=0.357462,A=1.000000)" 0.0 :!label _label)
  (Rendering|Debug|DrawDebugSphere _returnvalue_5 2e+02 12 "(R=1.000000,G=1.000000,B=1.000000,A=1.000000)" 0.0)
  (Utilities|FlowControl|Delay 2.0)
  (Actor|DestroyActor)
  (goto _label))

(event EventBeginPlay
  (Utilities|FlowControl|Delay 4.0)
  (Actor|DestroyActor))

(event Collision|EventActorBeginOverlap
  (params (OtherActor :type Actor%20Object%20Reference)))

(event EventTick
  (params (DeltaSeconds :type Float%20%28single-precision%29)))

(fn ConstructionScript)